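; Audio visualizer Blueprint that builds a centered row of mesh bars and can play a song on BeginPlay.
; The construction script spawns the bars along X from a count, spacing and shape, storing them in an array.
; Loops to scale the bars and feed Niagara vector parameters from a spectrum are disconnected, with no spectrum source.
; CalculateScale's offset-and-power Z scaling is also unconnected, so nothing reacts to audio.
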(event EventBeginPlay
  (if (Variables|Default|GetPlaySong)
    (Audio|Components|Audio|Play (Variables|Default|GetVibeAudio) 0.0)))

(event Collision|EventActorBeginOverlap
  (params (OtherActor :type Actor%20Object%20Reference)))

(event EventTick
  (params (DeltaSeconds :type Float%20%28single-precision%29)))

(fn ConstructionScript
  (bind _equalizernumber (Variables|Default|GetEqualizerNumber))
  (bind _equalizerspacing (Variables|Default|GetEqualizerSpacing))
  (bind _returnvalue (- _equalizernumber 1))
  (for _index (range 0 _returnvalue)
    (bind _returnvalue_2 (AddComponent|AddStaticMeshComponent false (Math|Transform|MakeTransform (Math|Vector|MakeVector (- (* _index _equalizerspacing) (/ (* _returnvalue _equalizerspacing) 2.0)) 0.0 0.0))))
    (Components|StaticMesh|SetStaticMesh _returnvalue_2 (Variables|Default|GetEqualizerShape))
    (Utilities|Array|Add (Variables|Default|GetEqualizerArray) _returnvalue_2)))