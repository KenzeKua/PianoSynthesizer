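; Audio visualizer actor that drives a Niagara grid from AudioSynesthesia Constant-Q analysis of a song.
; BeginPlay sets the sound, grid counts and spacing, and creates dynamic materials for two indicator lights.
; Overlapping the button volume enables input, letting E start or toggle pause with indicator feedback.
; Playback-percent callbacks sample the precomputed spectrum at the current time, pushing scaled and normalized arrays to Niagara.
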(event OnComponentBeginOverlap(ButtonCollision)
  (params (OverlappedComponent :type Primitive%20Component%20Object%20Reference) (OtherActor :type Actor%20Object%20Reference) (OtherComp :type Primitive%20Component%20Object%20Reference) (OtherBodyIndex :type Integer) (bFromSweep :type Boolean) (SweepResult :type Hit%20Result%20Structure%20%28by%20ref%29))
  (bind _returnvalue (Game|GetPlayerController 0))
  (Development|PrintString "Entered")
  (if (== (Game|GetInstigatorController (Components|GetOwner OtherActor)) (Game|GetInstigatorController _returnvalue))
    (Input|EnableInput _returnvalue)
    (Rendering|Material|SetScalarParameterValue (Variables|Default|GetEnterIndicatorDynamicMat) "Emission" 0.7 :!class /Script/Engine.MaterialInstanceDynamic)))

(event OnComponentEndOverlap(ButtonCollision)
  (params (OverlappedComponent :type Primitive%20Component%20Object%20Reference) (OtherActor :type Actor%20Object%20Reference) (OtherComp :type Primitive%20Component%20Object%20Reference) (OtherBodyIndex :type Integer))
  (bind _returnvalue (Game|GetPlayerController 0))
  (Development|PrintString "Exit")
  (if (== (Game|GetInstigatorController (Components|GetOwner OtherActor)) (Game|GetInstigatorController _returnvalue))
    (Input|DisableInput _returnvalue)
    (Rendering|Material|SetScalarParameterValue (Variables|Default|GetEnterIndicatorDynamicMat) "Emission" 0.0 :!class /Script/Engine.MaterialInstanceDynamic)))

(event Custom|UpdateSpectrum
  (params (PlayingSoundWave :type Sound%20Wave%20Object%20Reference) (PlaybackPercent :type Float%20%28single-precision%29))
  (bind _duration (Variables|/Script/Engine.SoundBase|GetDuration PlayingSoundWave))
  (bind _constq (Variables|Default|GetConstQ))
  (bind _vibeniagara (Variables|Default|GetVibeNiagara))
  (bind _returnvalue (* _duration PlaybackPercent))
  (bind _outconstantq (Class|ConstantQNRT|GetNormalizedChannelConstantQatTime _constq _returnvalue))
  (bind _output_get (Variables|Default|SetOut%20Spectrum _outconstantq))
  (CallFunction|CalculateScale _output_get)
  (Class|NiagaraDataInterfaceArrayFunctionLibrary|SetNiagaraArrayFloat _vibeniagara "User.OutSpectrum" (Variables|Default|GetOut%20Spectrum))
  (Class|NiagaraDataInterfaceArrayFunctionLibrary|SetNiagaraArrayFloat _vibeniagara "User.NormalizedSpectrum" _outconstantq))

(event EventBeginPlay
  (Audio|Components|Audio|SetSound (Variables|Default|GetVibeAudio) (Variables|/Script/AudioAnalyzer.AudioAnalyzerNRT|GetSound (Variables|Default|GetConstQ)))
  (CallFunction|SetNiagaraValues)
  (Utilities|FlowControl|Sequence
    (:then_0
      (bind _returnvalue (Rendering|Material|CreateDynamicMaterialInstance (Variables|Default|GetEnterIndicator) 0 "/Game/Art/MI_VisualizerIndicator1.MI_VisualizerIndicator1" "None" :!class /Script/Engine.PrimitiveComponent))
      (bind _output_get (Variables|Default|SetEnterIndicatorDynamicMat _returnvalue))
      (Rendering|Material|SetScalarParameterValue _output_get "Emission" 0.0 :!class /Script/Engine.MaterialInstanceDynamic)
      (Rendering|Material|SetVectorParameterValue _output_get "Colour" "(R=0.000000,G=0.345098,B=0.847059,A=1.000000)" :!class /Script/Engine.MaterialInstanceDynamic))
    (:then_1
      (bind _returnvalue_2 (Rendering|Material|CreateDynamicMaterialInstance (Variables|Default|GetPlayIndicator) 0 "/Game/Art/MI_VisualizerIndicator1.MI_VisualizerIndicator1" "None" :!class /Script/Engine.PrimitiveComponent))
      (bind _output_get_2 (Variables|Default|SetPlayIndicatorDynamicMat _returnvalue_2))
      (Rendering|Material|SetScalarParameterValue _output_get_2 "Emission" 0.7 :!class /Script/Engine.MaterialInstanceDynamic)
      (Rendering|Material|SetVectorParameterValue _output_get_2 "Colour" "(R=1.000000,G=0.000000,B=0.000000,A=1.000000)" :!class /Script/Engine.MaterialInstanceDynamic))))

(event Collision|EventActorBeginOverlap
  (params (OtherActor :type Actor%20Object%20Reference)))

(event EventTick
  (params (DeltaSeconds :type Float%20%28single-precision%29)))

(event Input|KeyboardEvents|E
  (params (Key :type Key%20Structure :default "None"))
  (bind _vibeaudio (Variables|Default|GetVibeAudio))
  (bind _playindicatordynamicmat (Variables|Default|GetPlayIndicatorDynamicMat))
  (:Pressed
    (if (Audio|Components|Audio|IsPlaying _vibeaudio)
      (Utilities|FlowControl|FlipFlop
        (:A
          (Class|AudioComponent|SetPaused _vibeaudio true)
          (Rendering|Material|SetVectorParameterValue _playindicatordynamicmat "Colour" "(R=1.000000,G=0.000000,B=0.000000,A=1.000000)" :!class /Script/Engine.MaterialInstanceDynamic))
        (:B
          (Class|AudioComponent|SetPaused _vibeaudio false)
          (Rendering|Material|SetVectorParameterValue _playindicatordynamicmat "Colour" "(R=0.129412,G=1.000000,B=0.000000,A=1.000000)" :!class /Script/Engine.MaterialInstanceDynamic :!label _label)))
      (else
        (EventDispatchers|AssignOnAudioPlaybackPercent _vibeaudio (delegate Custom|UpdateSpectrum))
        (if (Variables|Default|GetPlaySong)
          (Audio|Components|Audio|Play _vibeaudio 0.0)
          (goto _label))))))

(fn ConstructionScript)

(fn SetNiagaraValues
  (bind _vibeniagara (Variables|Default|GetVibeNiagara))
  (Niagara|SetNiagaraVariable(Float) _vibeniagara "User.XParticleCount" (Variables|Default|GetX%20Bar%20Count))
  (Niagara|SetNiagaraVariable(Float) _vibeniagara "User.YParticleCount" (Variables|Default|GetY%20Bar%20Count))
  (Niagara|SetNiagaraVariable(Float) _vibeniagara "User.ZParticleCount" (Variables|Default|GetZ%20Bar%20Count))
  (Niagara|SetNiagaraVariable(Float) _vibeniagara "User.ParticleStepSize" (Variables|Default|GetBarSpacing)))

(fn CalculateScale
  (params (In%20Spectrum :type Array%20of%20Floats%20%28double-precision%29))
  (for (_array_element _array_index) In%20Spectrum
    (Utilities|Array|SetArrayElem In%20Spectrum _array_index (* (+ _array_element (Variables|Default|GetSpectrum%20Offset)) (Variables|Default|GetSpectrum%20Power)))))