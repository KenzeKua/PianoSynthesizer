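; BP_MIDIController is a Blueprint that shows connected MIDI devices in a toggleable on-screen UI.
; On BeginPlay it enables player input, creates a hidden WBP_MainUI, and wraps each MIDI input device in a UO_DeviceInfo object for the widget's list.
; The device check counts output devices although the list uses inputs, showing a no-device warning when no outputs exist.
; Tab flip-flops the UI's visibility.
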(event EventBeginPlay
  (Input|EnableInput (Game|GetPlayerController 0))
  (bind _returnvalue (UserInterface|CreateWidget "/Game/UserInterface/WBP_MainUI.WBP_MainUI_C" (Game|GetPlayerController 0)))
  (bind _output_get (Variables|Default|SetMainUI _returnvalue))
  (UserInterface|Viewport|AddtoViewport _output_get 0)
  (Widget|SetVisibility _output_get "Hidden")
  (bind (_outmidiinputdevices _outmidioutputdevices) (Class|MIDIDeviceManager|FindAllMIDIDeviceInfo))
  (if (>= (Utilities|Array|Length _outmidioutputdevices) 1)
    (for _array_element _outmidiinputdevices
      (bind _returnvalue_2 (Game|ConstructObjectfromClass self "/Game/Blueprint/MIDI_Controller/UO_DeviceInfo.UO_DeviceInfo_C"))
      (Variables|/Game/Blueprint/MIDI_Controller/UO_DeviceInfo.UO_DeviceInfo_C|SetMIDI%20Device%20Info _returnvalue_2 (Utilities|Struct|MakeF_MIDIDeviceInfo (.DeviceID (Utilities|Struct|BreakMIDIDeviceInfo _array_element)) (.DeviceName (Utilities|Struct|BreakMIDIDeviceInfo _array_element)) (.bIsAlreadyInUse (Utilities|Struct|BreakMIDIDeviceInfo _array_element)) (.bIsDefaultDevice (Utilities|Struct|BreakMIDIDeviceInfo _array_element))))
      (Default|AddObjecttoList (Variables|Default|GetMainUI) _returnvalue_2))
    (else
      (Widget|SetVisibility (Variables|/Game/UserInterface/WBP_MainUI.WBP_MainUI_C|GetNoDeviceWarning (Variables|Default|GetMainUI)) "Visible"))))

(event Collision|EventActorBeginOverlap
  (params (OtherActor :type Actor%20Object%20Reference)))

(event EventTick
  (params (DeltaSeconds :type Float%20%28single-precision%29)))

(event Input|KeyboardEvents|Tab
  (params (Key :type Key%20Structure :default "None"))
  (bind _mainui (Variables|Default|GetMainUI))
  (:Pressed
    (Utilities|FlowControl|FlipFlop
      (:A
        (Widget|SetVisibility _mainui "Visible"))
      (:B
        (Widget|SetVisibility _mainui "Hidden")))))

(fn ConstructionScript)