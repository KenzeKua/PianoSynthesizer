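; BP_Synthesizer is a walk-up playable synthesizer that enables keyboard input while the player overlaps its box collision.
; Piano-style letter keys look up notes in DT_MIDINoteValue, add the octave shift and drive a MetaSound's note, attack and release.
; The same note indexes spectrum arrays pushed to a Niagara piano indicator.
; Number keys shift octave or toggle movement lock, with emissive indicators showing zone entry and lock state.
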(event OnComponentBeginOverlap(BoxCollision)
  (params (OverlappedComponent :type Primitive%20Component%20Object%20Reference) (OtherActor :type Actor%20Object%20Reference) (OtherComp :type Primitive%20Component%20Object%20Reference) (OtherBodyIndex :type Integer) (bFromSweep :type Boolean) (SweepResult :type Hit%20Result%20Structure%20%28by%20ref%29))
  (Development|PrintString "Entered")
  (if (== (Game|GetInstigatorController (Components|GetOwner OtherActor)) (Game|GetInstigatorController (Game|GetPlayerController 0)))
    (Input|EnableInput (Game|GetPlayerController 0))
    (Rendering|Material|SetScalarParameterValue (Variables|Default|GetEnterIndicatorDynamicMat) "Emission" 0.7 :!class /Script/Engine.MaterialInstanceDynamic)))

(event OnComponentEndOverlap(BoxCollision)
  (params (OverlappedComponent :type Primitive%20Component%20Object%20Reference) (OtherActor :type Actor%20Object%20Reference) (OtherComp :type Primitive%20Component%20Object%20Reference) (OtherBodyIndex :type Integer))
  (Development|PrintString "Exit")
  (if (== (Game|GetInstigatorController (Components|GetOwner OtherActor)) (Game|GetInstigatorController (Game|GetPlayerController 0)))
    (Input|DisableInput (Game|GetPlayerController 0))
    (Rendering|Material|SetScalarParameterValue (Variables|Default|GetEnterIndicatorDynamicMat) "Emission" 0.0 :!class /Script/Engine.MaterialInstanceDynamic)
    (Class|AudioParameterControllerInterface|SetTriggerParameter (Variables|Default|GetMetaSound) "Trigger Release")
    (CallFunction|ResetNiagaraValues)))

(event EventBeginPlay
  (Utilities|FlowControl|Sequence
    (:then_0
      (bind _returnvalue (Rendering|Material|CreateDynamicMaterialInstance (Variables|Default|GetEnterIndicator) 0 "/Game/Art/MI_VisualizerIndicator1.MI_VisualizerIndicator1" "None" :!class /Script/Engine.PrimitiveComponent))
      (bind _output_get (Variables|Default|SetEnterIndicatorDynamicMat _returnvalue))
      (Rendering|Material|SetScalarParameterValue _output_get "Emission" 0.0 :!class /Script/Engine.MaterialInstanceDynamic)
      (Rendering|Material|SetVectorParameterValue _output_get "Colour" "(R=0.000000,G=0.345098,B=0.847059,A=1.000000)" :!class /Script/Engine.MaterialInstanceDynamic))
    (:then_1
      (bind _returnvalue_2 (Rendering|Material|CreateDynamicMaterialInstance (Variables|Default|GetLockIndicator) 0 "/Game/Art/MI_VisualizerIndicator1.MI_VisualizerIndicator1" "None" :!class /Script/Engine.PrimitiveComponent))
      (bind _output_get_2 (Variables|Default|SetLockIndicatorDynamicMat _returnvalue_2))
      (Rendering|Material|SetScalarParameterValue _output_get_2 "Emission" 0.7 :!class /Script/Engine.MaterialInstanceDynamic)
      (Rendering|Material|SetVectorParameterValue _output_get_2 "Colour" "(R=1.000000,G=0.000000,B=0.000000,A=1.000000)" :!class /Script/Engine.MaterialInstanceDynamic))))

(event Collision|EventActorBeginOverlap
  (params (OtherActor :type Actor%20Object%20Reference)))

(event EventTick
  (params (DeltaSeconds :type Float%20%28single-precision%29)))

(event Input|KeyboardEvents|W
  (params (Key :type Key%20Structure :default "None"))
  (bind _metasound (Variables|Default|GetMetaSound))
  (:Pressed
    (bind (_midi_note _index) (CallFunction|GetMIDINoteValue Key))
    (CallFunction|SetNiagaraValues _index 1.0 1.0)
    (Effects|Components|ParticleSystem|SetIntParameter _metasound "MIDI Note" _midi_note)
    (Class|AudioParameterControllerInterface|SetTriggerParameter _metasound "Trigger Attack"))
  (:Released
    (CallFunction|SetNiagaraValues _index 0.0 0.0)
    (Class|AudioParameterControllerInterface|SetTriggerParameter _metasound "Trigger Release")))

(event Input|KeyboardEvents|E
  (params (Key :type Key%20Structure :default "None"))
  (bind _metasound (Variables|Default|GetMetaSound))
  (:Pressed
    (bind (_midi_note _index) (CallFunction|GetMIDINoteValue Key))
    (CallFunction|SetNiagaraValues _index 1.0 1.0)
    (Effects|Components|ParticleSystem|SetIntParameter _metasound "MIDI Note" _midi_note)
    (Class|AudioParameterControllerInterface|SetTriggerParameter _metasound "Trigger Attack"))
  (:Released
    (CallFunction|SetNiagaraValues _index 0.0 0.0)
    (Class|AudioParameterControllerInterface|SetTriggerParameter _metasound "Trigger Release")))

(event Input|KeyboardEvents|K
  (params (Key :type Key%20Structure :default "None"))
  (bind _metasound (Variables|Default|GetMetaSound))
  (:Pressed
    (bind (_midi_note _index) (CallFunction|GetMIDINoteValue Key))
    (CallFunction|SetNiagaraValues _index 1.0 1.0)
    (Effects|Components|ParticleSystem|SetIntParameter _metasound "MIDI Note" _midi_note)
    (Class|AudioParameterControllerInterface|SetTriggerParameter _metasound "Trigger Attack"))
  (:Released
    (CallFunction|SetNiagaraValues _index 0.0 0.0)
    (Class|AudioParameterControllerInterface|SetTriggerParameter _metasound "Trigger Release")))

(event Input|KeyboardEvents|Y
  (params (Key :type Key%20Structure :default "None"))
  (bind _metasound (Variables|Default|GetMetaSound))
  (:Pressed
    (bind (_midi_note _index) (CallFunction|GetMIDINoteValue Key))
    (CallFunction|SetNiagaraValues _index 1.0 1.0)
    (Effects|Components|ParticleSystem|SetIntParameter _metasound "MIDI Note" _midi_note)
    (Class|AudioParameterControllerInterface|SetTriggerParameter _metasound "Trigger Attack"))
  (:Released
    (CallFunction|SetNiagaraValues _index 0.0 0.0)
    (Class|AudioParameterControllerInterface|SetTriggerParameter _metasound "Trigger Release")))

(event Input|KeyboardEvents|U
  (params (Key :type Key%20Structure :default "None"))
  (bind _metasound (Variables|Default|GetMetaSound))
  (:Pressed
    (bind (_midi_note _index) (CallFunction|GetMIDINoteValue Key))
    (CallFunction|SetNiagaraValues _index 1.0 1.0)
    (Effects|Components|ParticleSystem|SetIntParameter _metasound "MIDI Note" _midi_note)
    (Class|AudioParameterControllerInterface|SetTriggerParameter _metasound "Trigger Attack"))
  (:Released
    (CallFunction|SetNiagaraValues _index 0.0 0.0)
    (Class|AudioParameterControllerInterface|SetTriggerParameter _metasound "Trigger Release")))

(event Input|KeyboardEvents|1
  (params (Key :type Key%20Structure :default "None"))
  (:Pressed
    (Variables|Default|SetOctave (Math|Integer|Clamp(Integer) (- (Variables|Default|GetOctave) 12) -24 24))
    (Development|PrintString (Utilities|String|Append "Octave : " (Utilities|String|ToString(Integer) (Variables|Default|GetOctave))))))

(event Input|KeyboardEvents|2
  (params (Key :type Key%20Structure :default "None"))
  (:Pressed
    (Variables|Default|SetOctave (Math|Integer|Clamp(Integer) (+ (Variables|Default|GetOctave) 12) -24 24))
    (Development|PrintString (Utilities|String|Append "Octave : " (Utilities|String|ToString(Integer) (Variables|Default|GetOctave))))))

(event Input|KeyboardEvents|3
  (params (Key :type Key%20Structure :default "None"))
  (bind _returnvalue (Game|GetPlayerController 0))
  (bind _lockindicatordynamicmat (Variables|Default|GetLockIndicatorDynamicMat))
  (:Pressed
    (Utilities|FlowControl|FlipFlop
      (:A
        (Input|SetIgnoreMoveInput _returnvalue true)
        (Rendering|Material|SetVectorParameterValue _lockindicatordynamicmat "Colour" "(R=0.129412,G=1.000000,B=0.000000,A=1.000000)" :!class /Script/Engine.MaterialInstanceDynamic))
      (:B
        (Input|ResetIgnoreMoveInput _returnvalue)
        (Rendering|Material|SetVectorParameterValue _lockindicatordynamicmat "Colour" "(R=1.000000,G=0.000000,B=0.000000,A=1.000000)" :!class /Script/Engine.MaterialInstanceDynamic)))))

(event Input|KeyboardEvents|T
  (params (Key :type Key%20Structure :default "None"))
  (bind _metasound (Variables|Default|GetMetaSound))
  (:Pressed
    (bind (_midi_note _index) (CallFunction|GetMIDINoteValue Key))
    (CallFunction|SetNiagaraValues _index 1.0 1.0)
    (Effects|Components|ParticleSystem|SetIntParameter _metasound "MIDI Note" _midi_note)
    (Class|AudioParameterControllerInterface|SetTriggerParameter _metasound "Trigger Attack"))
  (:Released
    (CallFunction|SetNiagaraValues _index 0.0 0.0)
    (Class|AudioParameterControllerInterface|SetTriggerParameter _metasound "Trigger Release")))

(event Input|KeyboardEvents|A
  (params (Key :type Key%20Structure :default "None"))
  (bind _metasound (Variables|Default|GetMetaSound))
  (:Pressed
    (bind (_midi_note _index) (CallFunction|GetMIDINoteValue Key))
    (CallFunction|SetNiagaraValues _index 1.0 1.0)
    (Effects|Components|ParticleSystem|SetIntParameter _metasound "MIDI Note" _midi_note)
    (Class|AudioParameterControllerInterface|SetTriggerParameter _metasound "Trigger Attack"))
  (:Released
    (CallFunction|SetNiagaraValues _index 0.0 0.0)
    (Class|AudioParameterControllerInterface|SetTriggerParameter _metasound "Trigger Release")))

(event Input|KeyboardEvents|S
  (params (Key :type Key%20Structure :default "None"))
  (bind _metasound (Variables|Default|GetMetaSound))
  (:Pressed
    (bind (_midi_note _index) (CallFunction|GetMIDINoteValue Key))
    (CallFunction|SetNiagaraValues _index 1.0 1.0)
    (Effects|Components|ParticleSystem|SetIntParameter _metasound "MIDI Note" _midi_note)
    (Class|AudioParameterControllerInterface|SetTriggerParameter _metasound "Trigger Attack"))
  (:Released
    (CallFunction|SetNiagaraValues _index 0.0 0.0)
    (Class|AudioParameterControllerInterface|SetTriggerParameter _metasound "Trigger Release")))

(event Input|KeyboardEvents|D
  (params (Key :type Key%20Structure :default "None"))
  (bind _metasound (Variables|Default|GetMetaSound))
  (:Pressed
    (bind (_midi_note _index) (CallFunction|GetMIDINoteValue Key))
    (CallFunction|SetNiagaraValues _index 1.0 1.0)
    (Effects|Components|ParticleSystem|SetIntParameter _metasound "MIDI Note" _midi_note)
    (Class|AudioParameterControllerInterface|SetTriggerParameter _metasound "Trigger Attack"))
  (:Released
    (CallFunction|SetNiagaraValues _index 0.0 0.0)
    (Class|AudioParameterControllerInterface|SetTriggerParameter _metasound "Trigger Release")))

(event Input|KeyboardEvents|F
  (params (Key :type Key%20Structure :default "None"))
  (bind _metasound (Variables|Default|GetMetaSound))
  (:Pressed
    (bind (_midi_note _index) (CallFunction|GetMIDINoteValue Key))
    (CallFunction|SetNiagaraValues _index 1.0 1.0)
    (Effects|Components|ParticleSystem|SetIntParameter _metasound "MIDI Note" _midi_note)
    (Class|AudioParameterControllerInterface|SetTriggerParameter _metasound "Trigger Attack"))
  (:Released
    (CallFunction|SetNiagaraValues _index 0.0 0.0)
    (Class|AudioParameterControllerInterface|SetTriggerParameter _metasound "Trigger Release")))

(event Input|KeyboardEvents|G
  (params (Key :type Key%20Structure :default "None"))
  (bind _metasound (Variables|Default|GetMetaSound))
  (:Pressed
    (bind (_midi_note _index) (CallFunction|GetMIDINoteValue Key))
    (CallFunction|SetNiagaraValues _index 1.0 1.0)
    (Effects|Components|ParticleSystem|SetIntParameter _metasound "MIDI Note" _midi_note)
    (Class|AudioParameterControllerInterface|SetTriggerParameter _metasound "Trigger Attack"))
  (:Released
    (CallFunction|SetNiagaraValues _index 0.0 0.0)
    (Class|AudioParameterControllerInterface|SetTriggerParameter _metasound "Trigger Release")))

(event Input|KeyboardEvents|H
  (params (Key :type Key%20Structure :default "None"))
  (bind _metasound (Variables|Default|GetMetaSound))
  (:Pressed
    (bind (_midi_note _index) (CallFunction|GetMIDINoteValue Key))
    (CallFunction|SetNiagaraValues _index 1.0 1.0)
    (Effects|Components|ParticleSystem|SetIntParameter _metasound "MIDI Note" _midi_note)
    (Class|AudioParameterControllerInterface|SetTriggerParameter _metasound "Trigger Attack"))
  (:Released
    (CallFunction|SetNiagaraValues _index 0.0 0.0)
    (Class|AudioParameterControllerInterface|SetTriggerParameter _metasound "Trigger Release")))

(event Input|KeyboardEvents|J
  (params (Key :type Key%20Structure :default "None"))
  (bind _metasound (Variables|Default|GetMetaSound))
  (:Pressed
    (bind (_midi_note _index) (CallFunction|GetMIDINoteValue Key))
    (CallFunction|SetNiagaraValues _index 1.0 1.0)
    (Effects|Components|ParticleSystem|SetIntParameter _metasound "MIDI Note" _midi_note)
    (Class|AudioParameterControllerInterface|SetTriggerParameter _metasound "Trigger Attack"))
  (:Released
    (CallFunction|SetNiagaraValues _index 0.0 0.0)
    (Class|AudioParameterControllerInterface|SetTriggerParameter _metasound "Trigger Release")))

(fn ConstructionScript)

(fn GetMIDINoteValue
  (params (Key :type Key%20Structure :default "None"))
  (bind _returnvalue (Utilities|GetDataTableRow "/Game/Blueprint/MIDI_Controller/DT_MIDINoteValue.DT_MIDINoteValue" (Utilities|String|StringToName (Utilities|String|ToString(Text) (Class|KismetInputLibrary|KeyGetDisplayName Key))))
    (:then
      (Development|PrintString (Utilities|String|Append "Note name : " (Utilities|String|ToString(Name) (.NoteName (Utilities|Struct|BreakF_InputKeys _returnvalue))) " | MIDI value : " (Utilities|String|ToString(Integer) (.MIDIValue (Utilities|Struct|BreakF_InputKeys _returnvalue)))))
      (return (+ (.MIDIValue (Utilities|Struct|BreakF_InputKeys _returnvalue)) (Variables|Default|GetOctave)) (- (+ (.MIDIValue (Utilities|Struct|BreakF_InputKeys _returnvalue)) (Variables|Default|GetOctave)) 36)))))

(fn SetNiagaraValues
  (params (Index :type Integer) (OutSpectrum :type Float%20%28double-precision%29) (Normalized%20Spectrum :type Float%20%28double-precision%29))
  (bind _niagarapianoindicator (Variables|Default|GetNiagaraPianoIndicator))
  (bind _normalizedspectrum (Variables|Default|GetNormalizedSpectrum))
  (Utilities|FlowControl|Sequence
    (:then_0
      (Utilities|Array|SetArrayElem (Variables|Default|GetOutSpectrum) Index OutSpectrum)
      (Class|NiagaraDataInterfaceArrayFunctionLibrary|SetNiagaraArrayFloat _niagarapianoindicator "User.OutSpectrum" (Variables|Default|GetOutSpectrum)))
    (:then_1
      (Utilities|Array|SetArrayElem _normalizedspectrum Index Normalized%20Spectrum)
      (Class|NiagaraDataInterfaceArrayFunctionLibrary|SetNiagaraArrayFloat _niagarapianoindicator "User.NormalizedSpectrum" _normalizedspectrum))))

(fn ResetNiagaraValues
  (bind _normalizedspectrum (Variables|Default|GetNormalizedSpectrum))
  (bind _outspectrum (Variables|Default|GetOutSpectrum))
  (for (_ _array_index) _outspectrum
    (Utilities|Array|SetArrayElem _outspectrum _array_index 0.0))
  (Class|NiagaraDataInterfaceArrayFunctionLibrary|SetNiagaraArrayFloat (Variables|Default|GetNiagaraPianoIndicator) "User.OutSpectrum" _outspectrum)
  (for (_ _array_index_2) _normalizedspectrum
    (Utilities|Array|SetArrayElem _normalizedspectrum _array_index_2 0.0))
  (Class|NiagaraDataInterfaceArrayFunctionLibrary|SetNiagaraArrayFloat (Variables|Default|GetNiagaraPianoIndicator) "User.NormalizedSpectrum" _normalizedspectrum))